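; Game instance that handles the game's menu flow and level transitions.
; It lazily creates and caches main menu, settings, leaderboard, pause and confirmation widgets, then adds them to the viewport.
; Main and pause menu events switch input to UI-only, with pause also freezing the game.
; Resume restores game input, restart reloads M_Gameplay via the new-game event, and an accepted pause confirmation opens M_MainMenu.
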(event Custom|ShowMainMenu
  (bind _returnvalue (Game|GetPlayerController 0))
  (Utilities|IsValid (Variables|widgets|GetW_MainMenu)
    (:Is%20Valid
      _)
    (:Is%20Not%20Valid
      (bind _returnvalue_2 (UserInterface|CreateWidget "/Game/UI/MainMenu/W_MainMenu.W_MainMenu_C" _returnvalue))
      (Variables|widgets|SetW_MainMenu _returnvalue_2)))
  (UserInterface|Viewport|AddtoViewport (Variables|widgets|GetW_MainMenu) 0)
  (Input|SetInputModeUIOnly _returnvalue (Variables|widgets|GetW_MainMenu) "DoNotLock"))

(event Custom|Pause:Confirmation
  (Utilities|IsValid (Variables|widgets|GetW_Confirmation)
    (:Is%20Valid
      _)
    (:Is%20Not%20Valid
      (bind _returnvalue (UserInterface|CreateWidget "/Game/UI/PauseMenu/W_Confirmation.W_Confirmation_C" (Game|GetPlayerController 0)))
      (Variables|widgets|SetW_Confirmation _returnvalue)))
  (UserInterface|Viewport|AddtoViewport (Variables|widgets|GetW_Confirmation) 0)
  (Widget|RemovefromParent (Variables|widgets|GetW_PauseMenu)))

(event Custom|Pause:Confirmation_Accept
  (Game|OpenLevel(byName) "M_MainMenu"))

(event Custom|CreateNewGame
  (Input|SetInputModeGameOnly (Game|GetPlayerController 0))
  (Game|OpenLevel(byName) "M_Gameplay"))

(event Custom|ShowSettingsMenu
  (Utilities|IsValid (Variables|widgets|GetW_SettingsMenu)
    (:Is%20Valid
      _)
    (:Is%20Not%20Valid
      (bind _returnvalue (UserInterface|CreateWidget "/Game/UI/MainMenu/W_SettingsMenu.W_SettingsMenu_C" (Game|GetPlayerController 0)))
      (Variables|widgets|SetW_SettingsMenu _returnvalue)))
  (UserInterface|Viewport|AddtoViewport (Variables|widgets|GetW_SettingsMenu) 0))

(event Custom|Pause:Confirmation_Decline
  (Widget|RemovefromParent (Variables|widgets|GetW_Confirmation))
  (UserInterface|Viewport|AddtoViewport (Variables|widgets|GetW_PauseMenu) 0))

(event Custom|ShowLeaderBoardMenu
  (Utilities|IsValid (Variables|widgets|GetW_LeaderBoardMenu)
    (:Is%20Valid
      _)
    (:Is%20Not%20Valid
      (bind _returnvalue (UserInterface|CreateWidget "/Game/UI/MainMenu/W_LeaderBoardMenu.W_LeaderBoardMenu_C" (Game|GetPlayerController 0)))
      (Variables|widgets|SetW_LeaderBoardMenu _returnvalue)))
  (UserInterface|Viewport|AddtoViewport (Variables|widgets|GetW_LeaderBoardMenu) 0))

(event Custom|ShowPauseMenu
  (bind _returnvalue (Game|GetPlayerController 0))
  (Utilities|IsValid (Variables|widgets|GetW_PauseMenu)
    (:Is%20Valid
      _)
    (:Is%20Not%20Valid
      (bind _returnvalue_2 (UserInterface|CreateWidget "/Game/UI/PauseMenu/W_PauseMenu.W_PauseMenu_C" _returnvalue))
      (Variables|widgets|SetW_PauseMenu _returnvalue_2)))
  (UserInterface|Viewport|AddtoViewport (Variables|widgets|GetW_PauseMenu) 0)
  (Input|SetInputModeUIOnly _returnvalue (Variables|widgets|GetW_PauseMenu) "DoNotLock")
  (Game|SetGamePaused true))

(event Custom|PauseMenu:Resume
  (Widget|RemovefromParent (Variables|widgets|GetW_PauseMenu))
  (Game|SetGamePaused false)
  (Input|SetInputModeGameOnly (Game|GetPlayerController 0)))

(event Custom|PauseMenu:Restart
  (Widget|RemovefromParent (Variables|widgets|GetW_PauseMenu))
  (Game|SetGamePaused false)
  (CallFunction|CreateNewGame))